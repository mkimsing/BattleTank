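; Player controller for the tank game that creates and drives the player's UI: aiming HUD, damage overlay, time-dilation effect, pause menus and death screen.
; BeginPlay pre-creates overlays and collapsed menus, FoundAimingComponent builds the HUD, and damage or time-dilation events set overlay fades.
; Game mode respawns re-link the HUD's aiming component, set health from HPBeforeRespawn (cached max health) and rebind time dilation.
; The menu toggle and death screen pause the game.
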(event `self.FoundAimingComponent`
  (params (AimComponentRef :type "TankAimingComponent Object Reference"))
  ;[1 1 1] Player Main UI
  (bind _asbattle_tank_game_mode_bp (cast `/Game/Blueprints/BattleTankGameMode_BP` (`GameplayStatics.GetGameMode`)))
  (add `/Game/Blueprints/BattleTankGameMode_BP.Respawn_Dispatcher` _asbattle_tank_game_mode_bp (delegate `PlayerRespawned`))
  (bind _returnvalue (`|CreateWidget` "/Game/UI/PlayersUI_BP.PlayersUI_BP_C"))
  (set `/Game/UI/PlayersUI_BP.BP Aiming Component Ref` AimComponentRef _returnvalue)
  (`UserWidget.AddToViewport` _returnvalue 0)
  (`Widget.SetVisibility` _returnvalue "Hidden"))

(event `PlayerRespawned`
  (bind _returnvalue (`GameplayStatics.GetPlayerPawn` 0))
  ;[1 1 1] Player Main UI
  (set `/Game/UI/PlayersUI_BP.BP Aiming Component Ref` (`self.GetComponentByClass` _returnvalue "/Script/BattleTank.TankAimingComponent") (stale `self.FoundAimingComponent` _returnvalue))
  (bind _asplayer_tank_bp (cast `/Game/Tank/PlayerTank_BP` _returnvalue))
  ;[1 1 1] Time Dilation UI / VFX
  (`Tank.SetCurrentHealth` _asplayer_tank_bp (`self.HPBeforeRespawn`))
  (bind _asplayer_tank_bp_2 (cast `/Game/Tank/PlayerTank_BP` (`GameplayStatics.GetPlayerPawn` 0) :!label _label))
  (add `Tank.TimeDilationEvent` _asplayer_tank_bp_2 (delegate `Time Dilation Delegate`))
  (set `self.HPBeforeRespawn` (`Tank.GetMaxHealth` _asplayer_tank_bp_2)))

(event `self.ReceiveTick`
  (params (DeltaSeconds :type "Float (single-precision)"))
  ;[1 1 1] Player Main UI
  (bind _returnvalue (`GameplayStatics.GetCurrentLevelName` true))
  (if (`KismetStringLibrary.NotEqual_StrStr` _returnvalue "MainMenu")
    (`Widget.SetVisibility` (stale `self.FoundAimingComponent` _returnvalue) "Visible")))

(event `self.PlayerDeath`
  ;[1 1 1] Game Over / Death Screen UI
  (bind _returnvalue (`|CreateWidget` "/Game/UI/DeathScreen.DeathScreen_C"))
  (`GameplayStatics.SetGamePaused` true)
  (`UserWidget.AddToViewport` _returnvalue 0)
  (`WidgetBlueprintLibrary.SetInputMode_UIOnlyEx` self (`/Game/UI/DeathScreen.RetryButton` _returnvalue)))

(event `InputAction|Start Menu` :paused true
  (params (Key :type "Key Structure"))
  ;[1 1 1] Start Menu UI
  (:`Pressed`
    (bind _isa (`/Engine/EditorBlueprintResources/StandardMacros.FlipFlop`)
      (:`A`
        _)
      (:`B`
        _))
    (`self.Toggle Menu` _isa)))

(event `self.ReceiveBeginPlay`
  ;[1 1 1] On Hit Damage Overlay UI
  (bind _returnvalue (`|CreateWidget` "/Game/UI/DamageOverlay_BP.DamageOverlay_BP_C"))
  (`UserWidget.AddToViewport` _returnvalue 0)
  ;[1 1 1] Init Start Menu (Invis)
  (bind _returnvalue_2 (`|CreateWidget` "/Game/UI/StartMenu_BP.StartMenu_BP_C" (`GameplayStatics.GetPlayerController` 0)))
  (`Widget.SetVisibility` _returnvalue_2 "Collapsed")
  (`UserWidget.AddToViewport` _returnvalue_2 1)
  (set `self.StartMenu` _returnvalue_2)
  ;[1 1 1] Init Controls Menu(invis)
  (bind _returnvalue_3 (`|CreateWidget` "/Game/UI/ControlsInGameMenu_BP.ControlsInGameMenu_BP_C" (`GameplayStatics.GetPlayerController` 0)))
  (`Widget.SetVisibility` _returnvalue_3 "Collapsed")
  (`UserWidget.AddToViewport` _returnvalue_3 1)
  (set `self.ControlsMenu` _returnvalue_3)
  ;[1 1 1] Time Dilation UI / VFX
  (bind _returnvalue_4 (`|CreateWidget` "/Game/UI/TimeDilationUI_BP.TimeDilationUI_BP_C" (`GameplayStatics.GetPlayerController` 0)))
  (`UserWidget.AddToViewport` _returnvalue_4 0)
  (`KismetSystemLibrary.Delay` 1.0)
  (goto _label))

(event `self.OnPlayerTankDamage`
  ;[1 1 1] On Hit Damage Overlay UI
  (set `/Game/UI/DamageOverlay_BP.Fade` 0.4 (stale `self.ReceiveBeginPlay` _returnvalue)) ; Starting Opacity for Damage Overlay
)

(event `Time Dilation Delegate`
  ;[1 1 1] Time Dilation UI / VFX
  (`self.Time Dilation VFX` (stale `self.ReceiveBeginPlay` _returnvalue_4)))

(fn `Time Dilation VFX`
  (params (`Time Dilation UI` :type "/Game/UI/TimeDilationUI_BP Object Reference"))
  (`/Engine/EditorBlueprintResources/StandardMacros.CompareFloat` (`GameplayStatics.GetGlobalTimeDilation`) 1.0
    (:`==`
      (set `/Game/UI/TimeDilationUI_BP.Fading IN` false `Time Dilation UI`)
      (set `/Game/UI/TimeDilationUI_BP.FadeOutFromOpacity` 0.5 `Time Dilation UI`))
    (:`<`
      (set `/Game/UI/TimeDilationUI_BP.Fading IN` true `Time Dilation UI`)
      (set `/Game/UI/TimeDilationUI_BP.FadeInFromOpactiy` 0.0 `Time Dilation UI`))))

(fn `Toggle Menu`
  (params (ShowMenu :type "Boolean (by ref)"))
  (bind _returnvalue (`GameplayStatics.GetPlayerController` 0))
  (bind _startmenu (`self.StartMenu`))
  (if ShowMenu
    (`Widget.SetVisibility` _startmenu "Visible")
    (`GameplayStatics.SetGamePaused` true)
    (`Widget.SetUserFocus` (`/Game/UI/StartMenu_BP.ControlsButton` _startmenu) _returnvalue)
    (else
      (`Widget.SetVisibility` _startmenu "Collapsed")
      (`Widget.SetVisibility` (`self.ControlsMenu`) "Collapsed")
      (`GameplayStatics.SetGamePaused` false)
      (`WidgetBlueprintLibrary.SetInputMode_GameOnly` _returnvalue))))

(fn `UserConstructionScript`)