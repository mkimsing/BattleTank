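; Player-controlled tank pawn that routes input to TankAiming and TankMovement for gimbal aiming, firing, reloading and track-driven movement, plus camera swap, boost and time dilation.
; BeginPlay and a post-respawn event share one init that wires barrel, turret, tracks, reload audio and health bar.
; Tick billboards the health bar and updates boost and dilation meters.
; Respawn saves transform to GameMode and health to PlayerController, then destroys spawned wheels and itself.
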(event `Re-Init after Respawn`
  (`TankAimingComponent.InitTurretComponents` (`self.TankAiming`) (`self.Barrel`) (`self.Turret`) :!label _label)
  (`TankMovementComponent.InitTracks` (`self.TankMovement`) (`self.Left Track`) (`self.Right Track`))
  (`self.Initialize Tank Heal Bar`)
  (`TankAimingComponent.InitAudioComponents` (`self.TankAiming`) (`self.ReloadSoundComponent`)))

(event `self.ReceiveBeginPlay`
  (goto _label))

(event `self.ReceiveTick`
  (params (DeltaSeconds :type "Float (single-precision)"))
  (`self.Rotate HP Bars to Camera`)
  (`self.ManageDilationMeter`)
  (`self.ManageBoostMeter`))

(event `InputAxis|AimAzimuth`
  (params (AxisValue :type "Float (single-precision)"))
  ;[1 1 1] Aiming/Firing Input Bindings
  (`SceneComponent.K2_AddLocalRotation` (`self.Azimuth Gimbal`) (`KismetMathLibrary.MakeRotator` 0.0 0.0 AxisValue) false false))

(event `InputAction|Quit`
  (params (Key :type "Key Structure"))
  ;[1 1 1] Aiming/Firing Input Bindings
  (:`Released`
    (`KismetSystemLibrary.QuitGame` null "Quit")))

(event `InputAxis|AimElevation`
  (params (AxisValue :type "Float (single-precision)"))
  ;[1 1 1] Aiming/Firing Input Bindings
  (`SceneComponent.K2_AddLocalRotation` (`self.SpringArm`) (`KismetMathLibrary.MakeRotator` 0.0 AxisValue) false false))

(event `InputAction|Fire`
  (params (Key :type "Key Structure"))
  ;[1 1 1] Aiming/Firing Input Bindings
  (:`Pressed`
    (`TankAimingComponent.Fire` (`self.TankAiming`))))

(event `InputAction|Swap Camera`
  (params (Key :type "Key Structure"))
  ;[1 1 1] Aiming/Firing Input Bindings
  (:`Pressed`
    (`SceneComponent.ToggleVisibility` (`self.HealthBar`) false)
    (`ActorComponent.ToggleActive` (`self.1st Person Camera`))
    (`ActorComponent.ToggleActive` (`self.3rd Person Camera`))))

(event `InputAction|Reload`
  (params (Key :type "Key Structure"))
  ;[1 1 1] Aiming/Firing Input Bindings
  (:`Pressed`
    (`TankAimingComponent.Reload` (`self.TankAiming`))))

(event `InputAction|TimeDilation`
  (params (Key :type "Key Structure"))
  ;[1 1 1] Aiming/Firing Input Bindings
  (:`Pressed`
    (`self.AttemptDilateTime`))
  (:`Released`
    (`self.ResumeTime`)))

(event `InputAction|Boost`
  (params (Key :type "Key Structure"))
  ;[1 1 1] Aiming/Firing Input Bindings
  (:`Pressed`
    (`self.StartBoost`))
  (:`Released`
    (`self.StopBoost`)))

(event `InputAction|Respawn`
  (params (Key :type "Key Structure"))
  (bind _returnvalue (`GameplayStatics.GetPlayerPawn` 0))
  ;[1 1 1] Aiming/Firing Input Bindings
  (:`Pressed`
    (bind _asbattle_tank_game_mode_bp (cast `/Game/Blueprints/BattleTankGameMode_BP` (`GameplayStatics.GetGameMode`)))
    (set `/Game/Blueprints/BattleTankGameMode_BP.PlayerTransform` (`self.GetTransform` _returnvalue) _asbattle_tank_game_mode_bp)
    (bind _astank_player_controller_bp (cast `/Game/Tank/TankPlayerController_BP` (`GameplayStatics.GetPlayerController` 0)))
    (bind _asplayer_tank_bp (cast `/Game/Tank/PlayerTank_BP` _returnvalue))
    (set `/Game/Tank/TankPlayerController_BP.HPBeforeRespawn` (`self.GetCurrentHealth` _asplayer_tank_bp) _astank_player_controller_bp)
    (`self.DeleteSpawnedWheels`)
    (`self.K2_DestroyActor`)))

(event `InputAxis|Move Forward`
  (params (AxisValue :type "Float (single-precision)"))
  ;[1 1 1] Movement Controls
  (`TankMovementComponent.IntendMoveForward` (`self.TankMovement`) AxisValue))

(event `InputAxis|Turn Right`
  (params (AxisValue :type "Float (single-precision)"))
  ;[1 1 1] Movement Controls
  (`TankMovementComponent.IntendTurnRight` (`self.TankMovement`) AxisValue))

(fn `DeleteSpawnedWheels`
  (for _array_element (`TankTrack.GetWheels` (`self.Right Track`))
    (`self.K2_DestroyActor` _array_element))
  (for _array_element_2 (`TankTrack.GetWheels` (`self.Left Track`))
    (`self.K2_DestroyActor` _array_element_2)))

(fn `Initialize Tank Heal Bar`
  (bind _ashealthbar (cast `/Game/UI/Healthbar` (`WidgetComponent.GetUserWidgetObject` (`self.HealthBar`))))
  (set `/Game/UI/Healthbar.MyTank` self _ashealthbar))

(fn `Rotate HP Bars to Camera`
  (bind _healthbar (`self.HealthBar`))
  (`SceneComponent.K2_SetWorldRotation` _healthbar (`KismetMathLibrary.FindLookAtRotation` (`SceneComponent.K2_GetComponentLocation` _healthbar) (`PlayerCameraManager.GetCameraLocation` (`GameplayStatics.GetPlayerCameraManager` 0))) false false))

(fn `UserConstructionScript`)