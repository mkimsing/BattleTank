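; Trigger volume that spawns a set number of Tank_BP actors at SpawnLocation the first time anything overlaps its TriggerBox.
; Each loop pass activates the Siren and Fire effects, then spawns a tank.
; A Delay inside the loop precedes deactivating Fire, but does not pause the loop, so spawns are not staggered.
; BeginPlay positions Fire just above the spawn point.
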(event `self.TriggerBox.OnComponentBeginOverlap`
  (params (OverlappedComponent :type "PrimitiveComponent Object Reference") (OtherActor :type "Actor Object Reference") (OtherComp :type "PrimitiveComponent Object Reference") (OtherBodyIndex :type Integer) (bFromSweep :type Boolean) (SweepResult :type "HitResult Structure (by ref)"))
  (`/Engine/EditorBlueprintResources/StandardMacros.DoOnce` false
    (:`Completed`
      (for _ (range 1 (+ (`self.NumSpawns`) 1))
        (`ActorComponent.Activate` (`self.Siren`) false)
        (`ActorComponent.Activate` (`self.Fire`) false)
        (`|SpawnActorFromClass` "/Game/Tank/Tank_BP.Tank_BP_C" (`KismetMathLibrary.MakeTransform` (`self.SpawnLocation`)) "Undefined" "OverrideRootScale" null null)
        (`KismetSystemLibrary.Delay` 2.5)
        (`ActorComponent.Deactivate` (`self.Fire`))))))

(event `self.ReceiveBeginPlay`
  (bind (_spawnlocation_x _spawnlocation_y _spawnlocation_z) (`KismetMathLibrary.BreakVector` (`self.SpawnLocation`)))
  (`SceneComponent.K2_SetWorldLocation` (`self.Fire`) (`KismetMathLibrary.MakeVector` _spawnlocation_x _spawnlocation_y (+ _spawnlocation_z 100.0)) false false))

(fn `UserConstructionScript`)