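; Game mode for a tank battle game that tracks remaining enemies, handles player respawn and drives slow-motion audio.
; When enemies run out, it shows the win screen on BattleGround or the level-complete screen elsewhere.
; On player destruction, it spawns and possesses a new tank after a delay, rebinds its events and fires a respawn dispatcher.
; The tank's time dilation event toggles music volume, global pitch, heartbeat and transition sounds.
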(event `Reset After Respawn`
  (bind _asplayer_tank_bp (cast `/Game/Tank/PlayerTank_BP` (`GameplayStatics.GetPlayerPawn` 0) :!label _label))
  (add `Tank.TimeDilationEvent` _asplayer_tank_bp (delegate `TimeDilationEventDelegate`))
  ;[1 1 1] Respawn Binding
  (bind _asplayer_tank_bp_2 (cast `/Game/Tank/PlayerTank_BP` (`Controller.K2_GetPawn` (`GameplayStatics.GetPlayerController` 0))))
  (add `Actor.OnDestroyed` _asplayer_tank_bp_2 (delegate `Respawn`)))

(event `self.ReceiveBeginPlay`
  (set `self.EnemiesLeft` (`self.MaxEnemies`))
  (`AudioComponent.Play` (`self.BG Music`) 0.0)
  (`self.InitLevelNamesArray`)
  (`KismetSystemLibrary.Delay` 1.0)
  (goto _label))

(event `AnEnemyDied`
  ;[1 1 1] Win / Advance Screen UI
  (bind _result (`/Engine/EditorBlueprintResources/StandardMacros.DecrementFloat` (`self.EnemiesLeft`))
    (:`  `
      (bind _output_get (set `self.EnemiesLeft` _result))
      (if (<= _output_get 0.0)
        (bind _returnvalue (`GameplayStatics.GetCurrentLevelName` true))
        (if (`KismetStringLibrary.EqualEqual_StrStr` _returnvalue "BattleGround")
          (`self.DisplayWinScreen`)
          (else
            (`self.DisplayLVLCompleteScreen`)))))))

(event `TimeDilationEventDelegate`
  ;[1 1 1] Time Dilation SFX
  (`self.TimeDilationSFX`))

(event `Respawn`
  (params (DestroyedActor :type "Actor Object Reference"))
  (bind (_playertransform_location _playertransform_rotation _playertransform_scale) (`KismetMathLibrary.BreakTransform` (`self.PlayerTransform`)))
  ;[1 1 1] Respawn Implementation
  (`KismetSystemLibrary.Delay` 1.5)
  (bind _returnvalue (`|SpawnActorFromClass` "/Game/Tank/PlayerTank_BP.PlayerTank_BP_C" (`KismetMathLibrary.MakeTransform` _playertransform_location (struct) _playertransform_scale) "AdjustIfPossibleButAlwaysSpawn" "OverrideRootScale" null null))
  (`Controller.Possess` (`GameplayStatics.GetPlayerController` 0) _returnvalue)
  (`/Game/Tank/PlayerTank_BP.Re-Init after Respawn` _returnvalue)
  (`self.Reset After Respawn`)
  (`self.Respawn_Dispatcher`))

(fn `DisplayLVLCompleteScreen`
  (bind _returnvalue (`GameplayStatics.GetPlayerController` 0))
  (bind _returnvalue_2 (`|CreateWidget` "/Game/UI/LevelComplete_BP.LevelComplete_BP_C" _returnvalue))
  (`UserWidget.AddToViewport` _returnvalue_2 0)
  (`WidgetBlueprintLibrary.SetInputMode_UIOnlyEx` _returnvalue (`/Game/UI/LevelComplete_BP.AdvanceButton` _returnvalue_2)))

(fn `DisplayWinScreen`
  (bind _returnvalue (`GameplayStatics.GetPlayerController` 0))
  (bind _returnvalue_2 (`|CreateWidget` "/Game/UI/WinScreen.WinScreen_C" _returnvalue))
  (`UserWidget.AddToViewport` _returnvalue_2 0)
  (`WidgetBlueprintLibrary.SetInputMode_UIOnlyEx` _returnvalue (`/Game/UI/WinScreen.RetryButton` _returnvalue_2)))

(fn `InitLevelNamesArray`
  (set `self.Level Names` (`|MakeArray` "TrainingGround" "BattleGround" ""))
  (return))

(fn `TimeDilationSFX`
  (bind _bg_music (`self.BG Music`))
  (`/Engine/EditorBlueprintResources/StandardMacros.CompareFloat` (`GameplayStatics.GetGlobalTimeDilation`) 1.0
    (:`==`
      (`AudioComponent.Stop` (`self.Heartbeat`))
      (`AudioComponent.AdjustVolume` _bg_music 0.0 1.0)
      (`GameplayStatics.SetGlobalPitchModulation` 1.0)
      (`AudioComponent.Play` (`self.Time Resume Sound`) 0.0))
    (:`<`
      (`AudioComponent.AdjustVolume` _bg_music 0.0 0.25)
      (`GameplayStatics.SetGlobalPitchModulation` 0.5)
      (`AudioComponent.Play` (`self.Time Slow Sound`) 0.0)
      (`AudioComponent.Play` (`self.Heartbeat`) 0.0))))

(fn `UserConstructionScript`)