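; Projectile Blueprint that plays a flyby sound based on its distance from the first player's pawn.
; BeginPlay sets the play radius, and each Tick measures the distance from the collision mesh to that pawn.
; Audio restarts from the beginning on every tick where the distance is at or beyond the radius, with no one-shot guard.
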(event `self.ReceiveTick`
  (params (DeltaSeconds :type "Float (single-precision)"))
  (bind _returnvalue (`GameplayStatics.GetPlayerPawn` 0))
  (bind _collisionmesh (`self.CollisionMesh`))
  ;[1 1 1] Play Projectile Flyby Sound Play
  (if (`KismetSystemLibrary.IsValid` _collisionmesh)
    (if (`KismetSystemLibrary.IsValid` _returnvalue)
      (if (>= (`KismetMathLibrary.Abs` (`KismetMathLibrary.VSize` (- (`SceneComponent.K2_GetComponentLocation` _collisionmesh) (`self.K2_GetActorLocation` _returnvalue)))) (stale `self.ReceiveBeginPlay` _output_get))
        (`AudioComponent.Play` (`self.Audio`) 0.0)))))

(event `self.ReceiveBeginPlay`
  ;[1 1 1] Play Projectile Flyby Sound Play
  (bind _output_get (set `self.Play Radius` 10000.0)) ; Distance between projectile and player
)

(fn `UserConstructionScript`)