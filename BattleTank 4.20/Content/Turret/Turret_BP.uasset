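; Turret_BP is a turret actor that uses a tank aiming component, shows a health bar and plays a sound on death.
; On BeginPlay it passes the barrel, dome and reload audio to TankAiming, links itself to the Healthbar widget and binds Death to OnTankDeath.
; Each tick it rotates the health bar component to face the first player's camera.
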(event `self.ReceiveBeginPlay`
  (`TankAimingComponent.InitTurretComponents` (`self.TankAiming`) (`self.Barrel`) (`self.Dome`))
  (`self.Initialize Turret HP Bar`)
  (`TankAimingComponent.InitAudioComponents` (`self.TankAiming`) (`self.ReloadSoundComponent`))
  (add `self.OnTankDeath` (delegate `Death`)))

(event `Death`
  (`ActorComponent.Activate` (`self.DeathSound`) false))

(event `self.ReceiveTick`
  (params (DeltaSeconds :type "Float (single-precision)"))
  (`self.Rotate HP Bar to Camera`))

(fn `Initialize Turret HP Bar`
  (bind _ashealthbar (cast `/Game/UI/Healthbar` (`WidgetComponent.GetUserWidgetObject` (`self.HealthBar`))))
  (set `/Game/UI/Healthbar.MyTank` self _ashealthbar))

(fn `Rotate HP Bar to Camera`
  (bind _healthbar (`self.HealthBar`))
  (`SceneComponent.K2_SetWorldRotation` _healthbar (`KismetMathLibrary.FindLookAtRotation` (`SceneComponent.K2_GetComponentLocation` _healthbar) (`PlayerCameraManager.GetCameraLocation` (`GameplayStatics.GetPlayerCameraManager` 0))) false false))

(fn `UserConstructionScript`)