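; Game mode for a tank battle game that tracks remaining enemies and handles the win condition.
; On BeginPlay it sets the enemy counter to MaxEnemies and starts background music once.
; Each AnEnemyDied event decrements the counter, and at zero or below it shows the win screen.
; The win screen is added to the viewport with UI-only input focused on its retry button.
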(event `self.ReceiveBeginPlay`
  (set `self.EnemiesLeft` (`self.MaxEnemies`))
  (`/Engine/EditorBlueprintResources/StandardMacros.DoOnce` false
    (:`Completed`
      (`AudioComponent.Play` (`self.BG Music`) 0.0))))

(event `AnEnemyDied`
  (bind _result (`/Engine/EditorBlueprintResources/StandardMacros.DecrementFloat` (`self.EnemiesLeft`))
    (:`  `
      (bind _output_get (set `self.EnemiesLeft` _result))
      (if (<= _output_get 0.0)
        (`self.DisplayWinScreen`)))))

(fn `DisplayWinScreen`
  (bind _returnvalue (`GameplayStatics.GetPlayerController` 0))
  (bind _returnvalue_2 (`|CreateWidget` "/Game/UI/WinScreen.WinScreen_C" _returnvalue))
  (`UserWidget.AddToViewport` _returnvalue_2 0)
  (`WidgetBlueprintLibrary.SetInputMode_UIOnlyEx` _returnvalue (`/Game/UI/WinScreen.RetryButton` _returnvalue_2)))

(fn `UserConstructionScript`)