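; Player controller Blueprint for tanks that manages the player's UI and damage overlay.
; FoundAimingComponent creates the player UI widget and hands it the aiming component reference.
; Tick uses a self-resetting DoOnce to add that UI to the viewport once the level is BattleGround and the reference is valid.
; The damage overlay is added on BeginPlay, and OnPlayerTankDamage sets its starting fade opacity.
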(event `self.ReceiveTick`
  (params (DeltaSeconds :type "Float (single-precision)"))
  (`/Engine/EditorBlueprintResources/StandardMacros.DoOnce` false :!label _label
    (:`Completed`
      (bind _returnvalue (`GameplayStatics.GetCurrentLevelName` true))
      (if (and (`KismetStringLibrary.EqualEqual_StrStr` _returnvalue "BattleGround") (`KismetSystemLibrary.IsValid` (stale `self.FoundAimingComponent` _output_get)))
        (`UserWidget.AddToViewport` (stale `self.FoundAimingComponent` _returnvalue) 0)
        (else
          (goto _label :!via `Reset`))))))

(event `self.FoundAimingComponent`
  (params (AimComponentRef :type "TankAimingComponent Object Reference"))
  (bind _returnvalue (`|CreateWidget` "/Game/UI/PlayersUI_BP.PlayersUI_BP_C"))
  (bind _output_get (set `/Game/UI/PlayersUI_BP.BP Aiming Component Ref` AimComponentRef _returnvalue)))

(event `self.ReceiveBeginPlay`
  (bind _returnvalue (`|CreateWidget` "/Game/UI/DamageOverlay_BP.DamageOverlay_BP_C"))
  (`UserWidget.AddToViewport` _returnvalue 0))

(event `self.OnPlayerTankDamage`
  (set `/Game/UI/DamageOverlay_BP.Fade` 0.4 (stale `self.ReceiveBeginPlay` _returnvalue)) ; Starting Opacity for Damage Overlay
)

(fn `UserConstructionScript`)