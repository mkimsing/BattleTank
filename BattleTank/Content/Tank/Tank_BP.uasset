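; Player tank pawn Blueprint that wires its components together and routes input for driving, aiming, firing and camera switching.
; On BeginPlay it passes barrel and turret to TankAiming, tracks to TankMovement, and itself to the health bar widget.
; Movement axes feed TankMovement and Fire triggers TankAiming.
; Aim axes rotate an azimuth gimbal and spring arm separately, and Swap Camera toggles first and third person cameras.
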(event `self.ReceiveBeginPlay`
  (`TankAimingComponent.InitTurretComponents` (`self.TankAiming`) (`self.Barrel`) (`self.Turret`))
  (`TankMovementComponent.InitTracks` (`self.TankMovement`) (`self.Left Track`) (`self.Right Track`))
  (`self.Initialize Tank Heal Bar` self))

(event `InputAxis|AimAzimuth`
  (params (AxisValue :type "Float (single-precision)"))
  ;[1 1 1] Aiming/Firing Input Bindings
  (`SceneComponent.K2_AddLocalRotation` (`self.Azimuth Gimbal`) (`KismetMathLibrary.MakeRotator` 0.0 0.0 AxisValue) false false))

(event `InputAxis|Move Forward`
  (params (AxisValue :type "Float (single-precision)"))
  ;[1 1 1] Movement Controls
  (`TankMovementComponent.IntendMoveForward` (`self.TankMovement`) AxisValue))

(event `InputAxis|Turn Right`
  (params (AxisValue :type "Float (single-precision)"))
  ;[1 1 1] Movement Controls
  (`TankMovementComponent.IntendTurnRight` (`self.TankMovement`) AxisValue))

(event `InputAxis|AimElevation`
  (params (AxisValue :type "Float (single-precision)"))
  ;[1 1 1] Aiming/Firing Input Bindings
  (`SceneComponent.K2_AddLocalRotation` (`self.SpringArm`) (`KismetMathLibrary.MakeRotator` 0.0 AxisValue) false false))

(event `InputAction|Fire`
  (params (Key :type "Key Structure"))
  ;[1 1 1] Aiming/Firing Input Bindings
  (:`Pressed`
    (`TankAimingComponent.Fire` (`self.TankAiming`))))

(event `InputAction|Swap Camera`
  (params (Key :type "Key Structure"))
  ;[1 1 1] Aiming/Firing Input Bindings
  (:`Pressed`
    (`ActorComponent.ToggleActive` (`self.1st Person Camera`))
    (`ActorComponent.ToggleActive` (`self.3rd Person Camera`))))

(fn `Initialize Tank Heal Bar`
  (bind _ashealthbar (cast `/Game/UI/Healthbar` (`WidgetComponent.GetUserWidgetObject` (`self.Widget`))))
  (set `/Game/UI/Healthbar.MyTank` self _ashealthbar))

(fn `UserConstructionScript`)