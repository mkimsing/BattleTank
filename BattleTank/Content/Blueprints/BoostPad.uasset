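; BoostPad is a trigger pad that repeatedly boosts the player's tank while it overlaps the pad's Box.
; On begin overlap by player 0's PlayerTank_BP, BoostTracks starts fast looping timers that call "Boost" by name on the left and right tracks.
; End overlap clears both timers through the handles BoostTracks returned.
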(event `self.Box.OnComponentBeginOverlap`
  (params (OverlappedComponent :type "PrimitiveComponent Object Reference") (OtherActor :type "Actor Object Reference") (OtherComp :type "PrimitiveComponent Object Reference") (OtherBodyIndex :type Integer) (bFromSweep :type Boolean) (SweepResult :type "HitResult Structure (by ref)"))
  (if (== OtherActor (`GameplayStatics.GetPlayerPawn` 0))
    (bind _asplayer_tank_bp (cast `/Game/Tank/PlayerTank_BP` OtherActor))
    (bind (_ltracktimerhandle _rtracktimerhandle) (`self.BoostTracks` _asplayer_tank_bp))))

(event `self.Box.OnComponentEndOverlap`
  (params (OverlappedComponent :type "PrimitiveComponent Object Reference") (OtherActor :type "Actor Object Reference") (OtherComp :type "PrimitiveComponent Object Reference") (OtherBodyIndex :type Integer))
  (if (== OtherActor (`GameplayStatics.GetPlayerPawn` 0))
    (`KismetSystemLibrary.K2_ClearAndInvalidateTimerHandle` (stale `self.Box.OnComponentBeginOverlap` _rtracktimerhandle))
    (`KismetSystemLibrary.K2_ClearAndInvalidateTimerHandle` (stale `self.Box.OnComponentBeginOverlap` _ltracktimerhandle))))

(fn `BoostTracks`
  (params (PlayerTank_BP :type "/Game/Tank/PlayerTank_BP Object Reference"))
  (returns (LTrackTimerHandle :type "TimerHandle Structure") (RTrackTimerHandle :type "TimerHandle Structure"))
  (bind _returnvalue (`KismetSystemLibrary.K2_SetTimer` (`/Game/Tank/PlayerTank_BP.Left Track` PlayerTank_BP) "Boost" 0.1 true))
  (bind _returnvalue_2 (`KismetSystemLibrary.K2_SetTimer` (`/Game/Tank/PlayerTank_BP.Right Track` PlayerTank_BP) "Boost" 0.1 true))
  (return _returnvalue _returnvalue_2))

(fn `UserConstructionScript`)