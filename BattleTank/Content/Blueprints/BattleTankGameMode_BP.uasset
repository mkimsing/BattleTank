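; Game mode for a tank battle that runs background music, player respawning, the enemy count and the win screen.
; On BeginPlay it binds the player tank's destruction to a delayed respawn and possession at PlayerTransform.
; The tank's time-dilation event drives slow-motion feedback through global pitch, music ducking, heartbeat and transition sounds, and a fading overlay.
; AnEnemyDied counts down remaining enemies, then shows the win screen with UI-only input.
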(event `self.ReceiveBeginPlay`
  (set `self.EnemiesLeft` (`self.MaxEnemies`))
  (`AudioComponent.Play` (`self.BG Music`) 0.0)
  (bind _astank_bp (cast `/Game/Tank/Tank_BP` (`GameplayStatics.GetPlayerPawn` 0)))
  (add `Tank.TimeDilationEvent` _astank_bp (delegate `TimeDilationEventDelegate`))
  (bind _returnvalue (`|CreateWidget` "/Game/UI/TimeDilationUI_BP.TimeDilationUI_BP_C" (`GameplayStatics.GetPlayerController` 0)))
  (`UserWidget.AddToViewport` _returnvalue 0)
  (bind _astank_bp_2 (cast `/Game/Tank/Tank_BP` (`Controller.K2_GetPawn` (`GameplayStatics.GetPlayerController` 0))))
  (add `Actor.OnDestroyed` _astank_bp_2 (delegate `Respawn`)))

(event `TimeDilationEventDelegate`
  ;[1 1 1] Time Dilation SFX
  (`self.TimeDilationFX` (stale `self.ReceiveBeginPlay` _returnvalue)))

(event `Respawn`
  (params (DestroyedActor :type "Actor Object Reference"))
  (bind (_playertransform_location _playertransform_rotation _playertransform_scale) (`KismetMathLibrary.BreakTransform` (`self.PlayerTransform`)))
  (`KismetSystemLibrary.Delay` 1.5)
  (bind _returnvalue (`|SpawnActorFromClass` "/Game/Tank/Tank_BP.Tank_BP_C" (`KismetMathLibrary.MakeTransform` _playertransform_location (struct) _playertransform_scale) "AdjustIfPossibleButAlwaysSpawn" "OverrideRootScale" null null))
  (`Controller.Possess` (`GameplayStatics.GetPlayerController` 0) _returnvalue)
  (`/Game/Tank/Tank_BP.Respawned` _returnvalue))

(event `AnEnemyDied`
  ;[1 1 1] Win Screen UI
  (bind _result (`/Engine/EditorBlueprintResources/StandardMacros.DecrementFloat` (`self.EnemiesLeft`))
    (:`  `
      (bind _output_get (set `self.EnemiesLeft` _result))
      (if (<= _output_get 0.0)
        (`self.DisplayWinScreen`)))))

(fn `DisplayWinScreen`
  (bind _returnvalue (`GameplayStatics.GetPlayerController` 0))
  (bind _returnvalue_2 (`|CreateWidget` "/Game/UI/WinScreen.WinScreen_C" _returnvalue))
  (`UserWidget.AddToViewport` _returnvalue_2 0)
  (`WidgetBlueprintLibrary.SetInputMode_UIOnlyEx` _returnvalue (`/Game/UI/WinScreen.RetryButton` _returnvalue_2)))

(fn `TimeDilationFX`
  (params (Overlay :type "/Game/UI/TimeDilationUI_BP Object Reference"))
  (bind _bg_music (`self.BG Music`))
  (`/Engine/EditorBlueprintResources/StandardMacros.CompareFloat` (`GameplayStatics.GetGlobalTimeDilation`) 1.0
    (:`==`
      (`AudioComponent.Stop` (`self.Heartbeat`))
      (`AudioComponent.AdjustVolume` _bg_music 0.0 1.0)
      (`GameplayStatics.SetGlobalPitchModulation` 1.0)
      (`AudioComponent.Play` (`self.Time Resume Sound`) 0.0)
      (set `/Game/UI/TimeDilationUI_BP.Fading IN` false Overlay)
      (set `/Game/UI/TimeDilationUI_BP.FadeOutFromOpacity` 0.5 Overlay))
    (:`<`
      (`AudioComponent.AdjustVolume` _bg_music 0.0 0.25)
      (`GameplayStatics.SetGlobalPitchModulation` 0.5)
      (`AudioComponent.Play` (`self.Time Slow Sound`) 0.0)
      (`AudioComponent.Play` (`self.Heartbeat`) 0.0)
      (set `/Game/UI/TimeDilationUI_BP.Fading IN` true Overlay)
      (set `/Game/UI/TimeDilationUI_BP.FadeInFromOpactiy` 0.0 Overlay))))

(fn `UserConstructionScript`)