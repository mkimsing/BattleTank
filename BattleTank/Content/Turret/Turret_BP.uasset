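; Turret_BP is a turret actor that aims and fires through a TankAiming component and shows a health bar widget.
; On BeginPlay it hands the Barrel and Dome meshes and a reload sound component to TankAiming.
; It also casts its widget component's user widget to Healthbar and sets itself as that bar's MyTank reference.
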(event `self.ReceiveBeginPlay`
  (`TankAimingComponent.InitTurretComponents` (`self.TankAiming`) (`self.Barrel`) (`self.Dome`))
  (`self.Initialize Turret HP Bar`)
  (`TankAimingComponent.InitAudioComponents` (`self.TankAiming`) (`self.ReloadSoundComponent`)))

(fn `Initialize Turret HP Bar`
  (bind _ashealthbar (cast `/Game/UI/Healthbar` (`WidgetComponent.GetUserWidgetObject` (`self.Widget`))))
  (set `/Game/UI/Healthbar.MyTank` self _ashealthbar))

(fn `UserConstructionScript`)